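; BP_MovieBreak is an area actor that plays the destroyer cutscene when its exit-area event fires.
; Overlap switches BP_SplineCamera's air wall off; the exit event switches it back on and starts the level sequence, binding the MyAreaDestroyer actor by the "Destroyer" tag at runtime.
; When the sequence finishes, player input is re-enabled and BP_NEOGameMode blends the view back to the spline camera.
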(event `self.ReceiveBeginPlay`
  (`parent.ReceiveBeginPlay`))

(event `self.ReceiveActorBeginOverlap`
  (params (OtherActor :type "Actor Object Reference"))
  (`parent.ReceiveActorBeginOverlap` OtherActor)
  (bind _returnvalue (`GameplayStatics.GetActorOfClass` "/Game/0130/Blueprints/BP_SplineCamera.BP_SplineCamera_C"))
  (`/Game/0130/Blueprints/BP_SplineCamera.AirWallSwitch` _returnvalue false))

(event `self.ExitAreaEvent`
  (bind _returnvalue (`GameplayStatics.GetActorOfClass` "/Game/0130/Blueprints/BP_SplineCamera.BP_SplineCamera_C"))
  (`/Game/0130/Blueprints/BP_SplineCamera.AirWallSwitch` _returnvalue true)
  (bind (_outactor _returnvalue_2) (`LevelSequencePlayer.CreateLevelSequencePlayer` "/Game/0102/Enemy/DestoroyerSequence.DestoroyerSequence" (make `MovieSceneSequencePlaybackSettings` false)))
  (add `MovieSceneSequencePlayer.OnFinished` _returnvalue_2 (delegate `CustomEvent`))
  (`|ExecutionSequence`
    (:`then_0`
      (bind _returnvalue_3 (`GameplayStatics.GetActorOfClass` "/Game/0102/MyAreaDestroyer.MyAreaDestroyer_C"))
      (`LevelSequenceActor.AddBindingByTag` _outactor "Destroyer" _returnvalue_3 false))
    (:`then_1`
      (`MovieSceneSequencePlayer.Play` (`LevelSequenceActor.SequencePlayer` _outactor)))))

(event `self.ReceiveEndPlay`
  (params (EndPlayReason :type "EEndPlayReason Enum" :default "Destroyed")))

(event `CustomEvent`
  (`self.EnableInput` (`GameplayStatics.GetPlayerCharacter` 0) null)
  (bind _returnvalue (`GameplayStatics.GetActorOfClass` "/Game/0130/Blueprints/BP_SplineCamera.BP_SplineCamera_C"))
  (bind _asbp_neogame_mode (cast `/Game/0122/Level/BP_NEOGameMode` (`GameplayStatics.GetGameMode`)))
  (`NEOGameMode.SetViewTargetWithBlend` _asbp_neogame_mode _returnvalue 1.0 "VTBlend_Linear" 0.0 false))

(fn `UserConstructionScript`
  (`parent.UserConstructionScript`))