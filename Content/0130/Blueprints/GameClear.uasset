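; GameClear is a trigger-volume actor that ends the game when the player enters it.
; When a PlayerCharacter overlaps its Box component, it fetches the game state through TGS_GameMode and sets IsGameOver to true.
; On BeginPlay it draws a long-lasting debug box to show the trigger volume in the world.
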(event `self.ReceiveBeginPlay`
  (bind _box (`self.Box`))
  (`KismetSystemLibrary.DrawDebugBox` (`PrimitiveComponent.GetCenterOfMass` _box "None") (`BoxComponent.BoxExtent` _box) (struct :`R` 0.892113 :`B` 0.586108 :`A` 1.0) (`self.K2_GetActorRotation`) 999.0 1.0))

(event `self.Box.OnComponentBeginOverlap`
  (params (OverlappedComponent :type "PrimitiveComponent Object Reference") (OtherActor :type "Actor Object Reference") (OtherComp :type "PrimitiveComponent Object Reference") (OtherBodyIndex :type Integer) (bFromSweep :type Boolean) (SweepResult :type "HitResult Structure (by ref)"))
  (cast `PlayerCharacter` OtherActor)
  (bind _astgs_game_mode (cast `TGS_GameMode` (`GameplayStatics.GetGameMode`)))
  (bind _returnvalue (`TGS_GameMode.GetGameState` _astgs_game_mode))
  (set `TGS_GameStateBase.bIsGameOver` true _returnvalue))

(fn `UserConstructionScript`)