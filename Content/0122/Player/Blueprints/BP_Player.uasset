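; Player Blueprint that shows or hides its Widget component depending on whether enemies are nearby.
; BeginPlay caches the player controller as BP_NEOPlayerController, and Tick polls its AnyEnemiesNearbyMoreSecond check.
; Two DoOnce gates reset each other, so visibility is set only when the check's result changes rather than every frame.
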(event `self.ReceiveBeginPlay`
  (bind _asbp_neoplayer_controller (cast `/Game/0122/Level/BP_NEOPlayerController` (`GameplayStatics.GetPlayerController` 0)))
  (set `self.As BP NEOPlayer Controller` _asbp_neoplayer_controller))

(event `self.ReceiveTick`
  (params (DeltaSeconds :type "Float (single-precision)"))
  (if (`NEOPlayerController.AnyEnemiesNearbyMoreSecond` (`self.As BP NEOPlayer Controller`))
    (`/Engine/EditorBlueprintResources/StandardMacros.DoOnce` false :!label _label
      (:`Completed`
        (`SceneComponent.SetVisibility` (`self.Widget`) true false)
        (goto _label_2 :!via `Reset`)))
    (else
      (`/Engine/EditorBlueprintResources/StandardMacros.DoOnce` false :!label _label_2
        (:`Completed`
          (`SceneComponent.SetVisibility` (`self.Widget`) false false)
          (goto _label :!via `Reset`))))))

(fn `UserConstructionScript`)