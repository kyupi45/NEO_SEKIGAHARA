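; BP_Lance is a lance that shows a pickup prompt when the player is near it.
; Each Tick it checks that the player is within pickup distance and that the lance is neither held nor falling.
; Two DoOnce nodes that reset each other act as an edge-triggered toggle, showing or hiding the Niagara effect and widget only when that condition changes.
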(event `self.ReceiveTick`
  (params (DeltaSeconds :type "Float (single-precision)"))
  (if (and (`self.GetIsPickUpDistanceEnteredPlayer`) (and (not (`self.GetIsHeld`)) (not (`self.GetIsFalling`))))
    (`/Engine/EditorBlueprintResources/StandardMacros.DoOnce` false :!label _label
      (:`Completed`
        (`SceneComponent.SetVisibility` (`self.Niagara`) true false)
        (`Widget.SetVisibility` (`WidgetComponent.GetWidget` (`self.Widget`)) "Visible")
        (goto _label_2 :!via `Reset`)))
    (else
      (`/Engine/EditorBlueprintResources/StandardMacros.DoOnce` false :!label _label_2
        (:`Completed`
          (`SceneComponent.SetVisibility` (`self.Niagara`) false false)
          (`Widget.SetVisibility` (`WidgetComponent.GetWidget` (`self.Widget`)) "Hidden")
          (goto _label :!via `Reset`))))))

(fn `UserConstructionScript`)