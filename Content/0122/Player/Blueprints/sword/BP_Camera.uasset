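; BP_Camera is a camera actor that adjusts its follow camera to whether the game is in a battle area.
; Every tick it looks up BP_TGS_GameStateBase and reads NowBattleArea, widening the FollowCamera field of view and clearing MCanMove in battle, restoring both otherwise.
; Its two cube components are hidden at start, and both branches switch off their collision.
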(event `self.ReceiveBeginPlay`
  (`SceneComponent.SetVisibility` (`self.Cube`) false false)
  (`SceneComponent.SetVisibility` (`self.Cube1`) false false))

(event `self.ReceiveTick`
  (params (DeltaSeconds :type "Float (single-precision)"))
  (bind _returnvalue (`GameplayStatics.GetActorOfClass` "/Game/0130/Blueprints/BP_TGS_GameStateBase.BP_TGS_GameStateBase_C"))
  (if (`TGS_GameStateBase.NowBattleArea` _returnvalue)
    (set `self.m_CanMove` false)
    (`PrimitiveComponent.SetCollisionEnabled` (`self.Cube`) "NoCollision")
    (`PrimitiveComponent.SetCollisionEnabled` (`self.Cube1`) "NoCollision")
    (`CameraComponent.SetFieldOfView` (`self.Follow_Camera`) 97.0)
    (else
      (set `self.m_CanMove` true)
      (`PrimitiveComponent.SetCollisionEnabled` (`self.Cube`) "NoCollision")
      (`PrimitiveComponent.SetCollisionEnabled` (`self.Cube1`) "NoCollision")
      (`CameraComponent.SetFieldOfView` (`self.Follow_Camera`) 90.0))))

(fn `UserConstructionScript`)